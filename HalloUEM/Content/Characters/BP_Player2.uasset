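; BP_Player2 is the second player's flipbook-sprite character, handling spawn placement and temporary invulnerability.
; Init gathers movement points tagged for Player 2 and teleports the character to the middle array entry, printing an error if none exist.
; MakeInvulnerable optionally shows the damaged flipbook, blinks the sprite via a timeline and starts a timer.
; MakeVulnerable ends the blink and restores a normal or stressed run flipbook based on remaining lives.
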(event EventMakeInvulnerable
  (params (bHasBeenDamaged :type Boolean))
  ;[1 1 1] Invulnerability
  (if bHasBeenDamaged
    (Sprite|SetFlipbook (Variables|Default|GetSprite) "/Game/Characters/BOY/Sprites/FLIPBOOKS/FB_Boy_damaged.FB_Boy_damaged"))
  (Utilities|Time|SetTimerbyEvent (delegate EventMakeVulnerable) (Variables|Default|GetTimeToBevulnerableAgain))
  (Variables|Default|SetbIsInvulnerable true)
  (Components|Timeline|SetPlayRate (Variables|Default|GetInvulnerabilityBlink) 5.0)
  (Timeline|InvulnerabilityBlink Play
    (:Update
      (Sprite|SetSpriteColor (Variables|Default|GetSprite)))))

(event Collision|EventActorBeginOverlap
  (params (OtherActor :type Actor%20Object%20Reference)))

(event EventTick
  (params (DeltaSeconds :type Float%20%28single-precision%29)))

(event EventMakeVulnerable
  ;[1 1 1] Invulnerability
  (if (<= (Variables|Default|GetNumberOfLifes) 1)
    (Sprite|SetFlipbook (Variables|Default|GetSprite) "/Game/Characters/BOY/Sprites/FLIPBOOKS/FB_Boy_RunStressed.FB_Boy_RunStressed")
    (else
      (Sprite|SetFlipbook (Variables|Default|GetSprite) "/Game/Characters/BOY/Sprites/FLIPBOOKS/FB_Boy_Run.FB_Boy_Run")))
  (Variables|Default|SetbIsInvulnerable false)
  (Audio|Components|Audio|Stop (Variables|Default|GetInvulnerabilityBlink))
  (Sprite|SetSpriteColor (Variables|Default|GetSprite) (Utilities|Struct|MakeLinearColor 1.0 1.0 1.0 1.0)))

(event EventBeginPlay)

(event EventInit
  (bind _outactors (Actor|GetAllActorswithTag "MovementPoint-Player2"))
  (if (> (Utilities|Array|Length _outactors) 0)
    (for _array_element _outactors
      (bind _asbp_player_movement_point (Utilities|Casting|CastToBP_PlayerMovementPoint _array_element))
      (Utilities|Array|Add (Variables|Default|GetMovementPoints) _asbp_player_movement_point))
    (Transformation|SetActorLocation (Transformation|GetActorLocation (Utilities|Array|Get(acopy) (Variables|Default|GetMovementPoints) (/ (Utilities|Array|Length (Variables|Default|GetMovementPoints)) 2))) false true)
    (else
      (Development|PrintString "Error. No Movement points found" true true "(R=1.000000,G=0.000000,B=0.000000,A=1.000000)" 1e+01))))

(fn ConstructionScript)