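; Actor component that triggers a player's current power-up or sabotage effect in a two-player game.
; UsePowerUp switches on CurrentPowerUp to step the owning character forward or temporarily slow that player's block manager.
; UseFuckedUp switches on CurrentFuckerUp to temporarily speed up the other player's blocks or blind that player.
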(event EventBeginPlay)

(event EventTick
  (params (DeltaSeconds :type Float%20%28single-precision%29)))

(event EventUsePowerUp
  (bind _playercharacter (Variables|Default|GetPlayerCharacter))
  (switch Utilities|FlowControl|Switch|SwitchonEnumPowerUpType (Variables|Default|GetCurrentPowerUp)
    (:DASH
      (Class|PlayerCharacter|StepForward _playercharacter))
    (:SLOW
      (Class|BlockManager|UpdateSpeed (Variables|/Script/HalloUEM.PlayerCharacter|GetBlockManager _playercharacter) false (Variables|Default|GetSlowTime)))))

(event EventUseFuckedUp
  (bind _playercharacter (Variables|Default|GetPlayerCharacter))
  (switch Utilities|FlowControl|Switch|SwitchonEnumFuckUpType (Variables|Default|GetCurrentFuckerUp)
    (:SPEED
      (Class|BlockManager|UpdateSpeed (Variables|/Script/HalloUEM.PlayerCharacter|GetBlockManager (Variables|/Script/HalloUEM.PlayerCharacter|GetOtherPlayer _playercharacter)) true (Variables|Default|GetIncreaseSpeedTime)))
    (:BLIND
      (Class|PlayerCharacter|BlindOtherPlayer _playercharacter))))