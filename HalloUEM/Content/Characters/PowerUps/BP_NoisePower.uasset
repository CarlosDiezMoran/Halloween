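; BP_NoisePower is an actor that animates three Paper2D tile map layers as a flipbook-style loop, apparently the visual for a noise power-up.
; Tick accumulates delta time until it reaches TimeToSwitch, then resets the timer and hides all three tile maps.
; It advances a modulo-three layer index and unhides the matching tile map, so only one layer shows after each switch.
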(event EventBeginPlay)

(event Collision|EventActorBeginOverlap
  (params (OtherActor :type Actor%20Object%20Reference)))

(event EventTick
  (params (DeltaSeconds :type Float%20%28single-precision%29))
  (Variables|Default|SetCurrentTime (+ DeltaSeconds (Variables|Default|GetCurrentTime)))
  (if (>= (Variables|Default|GetCurrentTime) (Variables|Default|GetTimeToSwitch))
    (Variables|Default|SetCurrentTime 0.0)
    (Development|SetHiddeninGame (Variables|Default|GetPaperTileMap) true false)
    (Development|SetHiddeninGame (Variables|Default|GetPaperTileMap1) true false)
    (Development|SetHiddeninGame (Variables|Default|GetPaperTileMap2) true false)
    (bind _output_get (Variables|Default|SetCurrentlayer (Math|Integer|%(Integer) (+ (Variables|Default|GetCurrentlayer) 1) 3)))
    (switch int _output_get
      (:0
        (Development|SetHiddeninGame (Variables|Default|GetPaperTileMap) false false))
      (:1
        (Development|SetHiddeninGame (Variables|Default|GetPaperTileMap1) false false))
      (:2
        (Development|SetHiddeninGame (Variables|Default|GetPaperTileMap2) false false)))))

(fn ConstructionScript)