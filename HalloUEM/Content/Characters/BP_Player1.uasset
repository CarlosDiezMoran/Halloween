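; Player 1's flipbook sprite character, which starts on the middle of its tagged movement points and reacts to blocks and power-up props.
; Capsule overlap with a block triggers a step back; a prop grants a random power-up and "fuck-up" pair, excluding one power-up type at three lives.
; Temporary invulnerability uses a timer and a blinking timeline, swapping flipbooks for damage and low-life stress.
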(event OnComponentBeginOverlap(CapsuleComponent)
  (params (OverlappedComponent :type Primitive%20Component%20Object%20Reference) (OtherActor :type Actor%20Object%20Reference) (OtherComp :type Primitive%20Component%20Object%20Reference) (OtherBodyIndex :type Integer) (bFromSweep :type Boolean) (SweepResult :type Hit%20Result%20Structure%20%28by%20ref%29))
  (Utilities|Casting|CastToBlock OtherActor
    (:then
      (Class|PlayerCharacter|StepBack))
    (:CastFailed
      (bind _asbp_powerup_prop (Utilities|Casting|CastToBP_PowerupProp OtherActor))
      (if (== (Variables|Default|GetNumberOfLifes) 3)
        (Variables|Default|SetBytePowerUp (Math|Conversions|ToByte(Integer) (Math|Random|RandomIntegerinRange 2 3)))
        (else
          (Variables|Default|SetBytePowerUp (Math|Conversions|ToByte(Integer) (Math|Random|RandomIntegerinRange 1 3)))))
      (bind _output_get (Variables|Default|SetByteFuckerUp (Math|Conversions|ToByte(Integer) (Math|Random|RandomIntegerinRange 1 3))))
      (Class|PlayerCharacter|AddPowerUps (Utilities|Enum|ByteToEnumEnumPowerUpType (Variables|Default|GetBytePowerUp)) (Utilities|Enum|ByteToEnumEnumFuckUpType _output_get))
      (Variables|/Script/HalloUEM.AbilityProp|SetbHasToBeRemoved _asbp_powerup_prop true))))

(event EventMakeInvulnerable
  (params (bHasBeenDamaged :type Boolean))
  ;[1 1 1] Invulnerability
  (if bHasBeenDamaged
    (Sprite|SetFlipbook (Variables|Default|GetSprite) "/Game/Characters/GIRL/Sprites/FLIPBOOKS/FB_Girl_Damaged.FB_Girl_Damaged"))
  (Utilities|Time|SetTimerbyEvent (delegate EventMakeVulnerable) (Variables|Default|GetTimeToBevulnerableAgain))
  (Variables|Default|SetbIsInvulnerable true)
  (Components|Timeline|SetPlayRate (Variables|Default|GetInvulnerabilityBlink) 5.0)
  (bind _newtrack_0 (Timeline|InvulnerabilityBlink PlayFromStart)
    (:Update
      (Sprite|SetSpriteColor (Variables|Default|GetSprite) (Utilities|Struct|MakeLinearColor _newtrack_0 _newtrack_0 _newtrack_0 _newtrack_0)))))

(event Collision|EventActorBeginOverlap
  (params (OtherActor :type Actor%20Object%20Reference)))

(event EventMakeVulnerable
  ;[1 1 1] Invulnerability
  (if (<= (Variables|Default|GetNumberOfLifes) 1)
    (Sprite|SetFlipbook (Variables|Default|GetSprite) "/Game/Characters/GIRL/Sprites/FLIPBOOKS/FB_Girl_Stressed.FB_Girl_Stressed")
    (else
      (Sprite|SetFlipbook (Variables|Default|GetSprite) "/Game/Characters/GIRL/Sprites/FLIPBOOKS/FB_Girl_Normal.FB_Girl_Normal")))
  (Variables|Default|SetbIsInvulnerable false)
  (Audio|Components|Audio|Stop (Variables|Default|GetInvulnerabilityBlink))
  (Sprite|SetSpriteColor (Variables|Default|GetSprite) (Utilities|Struct|MakeLinearColor 1.0 1.0 1.0 1.0)))

(event EventInit
  (bind _outactors (Actor|GetAllActorswithTag "MovementPoint-Player1"))
  (if (> (Utilities|Array|Length _outactors) 0)
    (for _array_element _outactors
      (bind _asbp_player_movement_point (Utilities|Casting|CastToBP_PlayerMovementPoint _array_element))
      (Utilities|Array|Add (Variables|Default|GetMovementPoints) _asbp_player_movement_point))
    (Transformation|SetActorLocation (Transformation|GetActorLocation (Utilities|Array|Get(acopy) (Variables|Default|GetMovementPoints) (/ (Utilities|Array|Length (Variables|Default|GetMovementPoints)) 2))) false true)
    (else
      (Development|PrintString "Error. No Movement points found" true true "(R=1.000000,G=0.000000,B=0.000000,A=1.000000)" 1e+01))))

(fn ConstructionScript)